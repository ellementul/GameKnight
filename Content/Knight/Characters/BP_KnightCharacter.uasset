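; Player knight character Blueprint that handles horizontal movement, attacking, and syncing health and coins with the game instance.
; MoveRIght, MoveLeft and Stop events set a direction that Tick feeds into movement input, while releasing the Attack input calls ActionAttack.
; BeginPlay and OnHurted copy health and the character's coins to GI_Knight.
; ChangeCoins adds directly to the game instance's coin total and prints it.
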(event `self.ReceiveBeginPlay`
  (`self.UpdateHealth` :!label _label))

(event `self.OnHurted`
  (goto _label))

(event `self.ReceiveTick`
  (params (DeltaSeconds :type "Float (single-precision)"))
  (`self.AddMovementInput` (`KismetMathLibrary.MakeVector` (`self.MoveDirect`))))

(event `MoveRIght`
  (set `self.MoveDirect` 1.0))

(event `MoveLeft`
  (set `self.MoveDirect` -1.0))

(event `Stop`
  (set `self.MoveDirect` 0.0))

(event `InputAction|Attack`
  (params (Key :type "Key Structure"))
  (:`Released`
    (`self.ActionAttack` (0.0 0.0 0.0))))

(fn `ChangeCoins`
  (params (AddedCoins :type Integer))
  (bind _asgi_knight (cast `/Game/Knight/Blueprints/GI_Knight` (`GameplayStatics.GetGameInstance`)))
  (bind _output_get (set `/Game/Knight/Blueprints/GI_Knight.Coins` (+ (`/Game/Knight/Blueprints/GI_Knight.Coins` _asgi_knight) AddedCoins) _asgi_knight))
  (`KismetSystemLibrary.PrintString` (`KismetStringLibrary.Conv_IntToString` _output_get)))

(fn `UpdateHealth`
  (bind _returnvalue (`self.GetHealth`))
  (bind _asgi_knight (cast `/Game/Knight/Blueprints/GI_Knight` (`GameplayStatics.GetGameInstance`)))
  (set `/Game/Knight/Blueprints/GI_Knight.Health` _returnvalue _asgi_knight)
  (set `/Game/Knight/Blueprints/GI_Knight.Coins` (`self.Coins`) _asgi_knight))

(fn `UserConstructionScript`)