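; Pig character for the Knight game that extends a parent Blueprint and drops a loot actor when killed.
; Tick mirrors the IsSpeak flag onto the visibility of the Dirt component every frame.
; OnKilled clears IsSpeak, hiding Dirt on the next tick, and always spawns a Lut actor at the pig's location with IsMove enabled.
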(event `self.ReceiveBeginPlay`
  (`parent.ReceiveBeginPlay`))

(event `self.ReceiveTick`
  (params (DeltaSeconds :type "Float (single-precision)"))
  (`SceneComponent.SetVisibility` (`self.Dirt`) (`self.IsSpeak`) false)
  (`parent.ReceiveTick` DeltaSeconds))

(event `self.OnKilled`
  (set `self.IsSpeak` false)
  (`|SpawnActorFromClass` (`self.Lut`) (`KismetMathLibrary.MakeTransform` (`self.K2_GetActorLocation`)) "AlwaysSpawn" "OverrideRootScale" null true null))

(fn `UserConstructionScript`
  (`parent.UserConstructionScript`))