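; GenTiles is an actor that procedurally generates a tile map through its GenerationTileMap component and populates it with actors.
; The construction script passes the starting map, patterns, triggers and an error tile to that component.
; On BeginPlay it runs generation, then spawns each returned bind actor class at its location offset by the actor's own position.
; Gen and Clear functions wrap the component's generation and clearing.
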(event `self.ReceiveBeginPlay`
  (`GenerationTileMapComponent.Generation` (`self.GenerationTileMap`))
  (bind _returnvalue (`GenerationTileMapComponent.GetBindActors` (`self.GenerationTileMap`)))
  (for _array_element _returnvalue
    (bind (_classactor _location) (break `ActorSpawning` _array_element))
    (`|SpawnActorFromClass` _classactor (`KismetMathLibrary.MakeTransform` (+ _location (`self.K2_GetActorLocation`))) "AlwaysSpawn" "OverrideRootScale" self null)))

(fn `Clear`
  (`GenerationTileMapComponent.Clear` (`self.GenerationTileMap`)))

(fn `Gen`
  (`GenerationTileMapComponent.Generation` (`self.GenerationTileMap`)))

(fn `UserConstructionScript`
  (bind _generationtilemap (`self.GenerationTileMap`))
  (`PaperTileMapComponent.SetTileMap` _generationtilemap (`self.BeginMap`))
  (set `GenerationTileMapComponent.TilePatterns` (`self.Patterns`) _generationtilemap)
  (set `GenerationTileMapComponent.ErrorTile` (`TileMapBlueprintLibrary.MakeTile` 0 (`self.ErrorTileSet`)) _generationtilemap)
  (set `GenerationTileMapComponent.Triggers` (`self.Triggers`) _generationtilemap))