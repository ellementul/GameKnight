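; GM_Knight is the Knight game mode that owns the player HUD, pause menu and current cutscene reference.
; On BeginPlay it creates both widgets, keeping the pause menu hidden.
; Pause and unpause events toggle menu visibility, mouse cursor and game pause state, while an exit event quits the game.
; SetCutScene accepts a cutscene only when no valid one is stored, returning whether it was accepted.
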(event `self.ReceiveBeginPlay`
  (`|ExecutionSequence`
    (:`then_0`
      (bind _returnvalue (`|CreateWidget` "/Game/Knight/UI/WBP_PauseMenu.WBP_PauseMenu_C"))
      (`UserWidget.AddToViewport` _returnvalue 0)
      (bind _output_get (set `self.PauseMenu` _returnvalue))
      (`Widget.SetVisibility` _returnvalue "Hidden")
      (`Widget.SetVisibility` _output_get "Hidden"))
    (:`then_1`
      (bind _returnvalue_2 (`|CreateWidget` "/Game/Knight/UI/WBP_HUD.WBP_HUD_C"))
      (`UserWidget.AddToViewport` _returnvalue_2 0)
      (set `self.PlayrHUD` _returnvalue_2))))

(event `OnPause`
  (`Widget.SetVisibility` (`self.PauseMenu`) "Visible")
  (set `PlayerController.bShowMouseCursor` true (`GameplayStatics.GetPlayerController` 0))
  (`GameplayStatics.SetGamePaused` true)
  (set `self.IsPaused` true))

(event `OnUnpause`
  (`Widget.SetVisibility` (`self.PauseMenu`) "Hidden")
  (set `PlayerController.bShowMouseCursor` false (`GameplayStatics.GetPlayerController` 0))
  (`GameplayStatics.SetGamePaused` false)
  (set `self.IsPaused` false))

(event `OnExit`
  (`KismetSystemLibrary.QuitGame` null "Quit"))

(fn `GetCutScene`
  (returns (CurrentCutScene :type "/Game/Knight/Blueprints/BP_Cutscene Object Reference"))
  (return (`self.CurrentCutScene`)))

(fn `IsCutScene`
  (returns (IsScene :type Boolean))
  (return (`KismetSystemLibrary.IsValid` (`self.CurrentCutScene`))))

(fn `SetCutScene`
  (params (CurrentCutScene :type "/Game/Knight/Blueprints/BP_Cutscene Object Reference"))
  (returns (IsSetup :type Boolean))
  (locals (IsLocalSetup :type Boolean :default false))
  (bind _returnvalue (not (`self.IsCutScene`)))
  (set `local.IsLocalSetup` _returnvalue)
  (if _returnvalue
    (set `self.CurrentCutScene` CurrentCutScene))
  (return (`local.IsLocalSetup`)))

(fn `UserConstructionScript`)